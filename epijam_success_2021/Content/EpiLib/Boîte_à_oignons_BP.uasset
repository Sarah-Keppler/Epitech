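; Onion box Actor (Boîte à oignons) for what appears to be a cooking game, showing its held item through the MiniSosoh sprite.
; Every Tick, ObjetPrésent toggles the sprite tint between opaque white and, apparently, transparent.
; When present, a nested priority chain of item booleans (photos, plates, soup, vegetables, plated dishes) calls SetSprite, though no sprite assets are specified.
; Nothing here sets those flags or handles interaction.
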(event EventBeginPlay)

(event Collision|EventActorBeginOverlap
  (params (OtherActor :type Actor%20Object%20Reference)))

(event EventTick
  (params (DeltaSeconds :type Float%20%28single-precision%29))
  (if (Variables|Default|GetObjet%20présent%20?)
    (Sprite|SetSpriteColor (Variables|Default|GetMiniSosoh) (Utilities|Struct|MakeLinearColor 1.0 1.0 1.0 1.0))
    (if (Variables|Default|GetPhoto%20?)
      (Rendering|Components|Sprite|SetSprite (Variables|Default|GetMiniSosoh) 0)
      (elif (Variables|Default|GetPhoto%20découpé%20?)
        (Rendering|Components|Sprite|SetSprite (Variables|Default|GetMiniSosoh) 0)
        (elif (Variables|Default|GetAssiette%20?)
          (Rendering|Components|Sprite|SetSprite (Variables|Default|GetMiniSosoh) 0)
          (elif (Variables|Default|GetAssiette%20sale%20?)
            (Rendering|Components|Sprite|SetSprite (Variables|Default|GetMiniSosoh) 0)
            (elif (Variables|Default|GetSoupe%20de%20photos%20?)
              (Rendering|Components|Sprite|SetSprite (Variables|Default|GetMiniSosoh) 0)
              (elif (Variables|Default|GetTomate%20?)
                (Rendering|Components|Sprite|SetSprite (Variables|Default|GetMiniSosoh) 0)
                (elif (Variables|Default|GetSalade%20?)
                  (Rendering|Components|Sprite|SetSprite (Variables|Default|GetMiniSosoh) 0)
                  (elif (Variables|Default|GetAssiette%20de%20tomates%20?)
                    (Rendering|Components|Sprite|SetSprite (Variables|Default|GetMiniSosoh) 0)
                    (elif (Variables|Default|GetAssiette%20de%20salades%20?)
                      (Rendering|Components|Sprite|SetSprite (Variables|Default|GetMiniSosoh) 0)
                      (elif (Variables|Default|GetAssiette%20de%20tomate-salades%20?)
                        (Rendering|Components|Sprite|SetSprite (Variables|Default|GetMiniSosoh) 0)))))))))))
    (else
      (Sprite|SetSpriteColor (Variables|Default|GetMiniSosoh) (Utilities|Struct|MakeLinearColor 1.0 1.0 1.0 0.0)))))

(fn ConstructionScript)