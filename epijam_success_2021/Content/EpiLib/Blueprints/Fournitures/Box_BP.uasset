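; Box_BP is a supply box that hands out a Transportable item, apparently built on a table-like parent.
; TakeContent returns whatever TakeOnTheTable gives when an Object is present; otherwise it returns a fresh copy of TransportableToTake, so the supply never depletes.
; BeginPlay only calls the parent, and the logic that would set the sprite from the item's Image is disconnected.
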(event EventBeginPlay
  (|CallParentFunction))

(event Collision|EventActorBeginOverlap
  (params (OtherActor :type Actor%20Object%20Reference))
  (|CallParentFunction OtherActor) ; This node is disabled and will not be called.\nDrag off pins to build functionality.
)

(event EventTick
  (params (DeltaSeconds :type Float%20%28single-precision%29))
  (|CallParentFunction DeltaSeconds) ; This node is disabled and will not be called.\nDrag off pins to build functionality.
)

(fn ConstructionScript
  (|CallParentFunction))

(fn TakeContent
  (bind _transportabletotake (Variables|Default|GetTransportableToTake))
  (if (Utilities|IsValid (Variables|Default|GetObject))
    (bind _content (CallFunction|TakeontheTable))
    (return _content)
    (else
      (bind _copy (Default|GetACopy _transportabletotake _transportabletotake))
      (return _copy))))