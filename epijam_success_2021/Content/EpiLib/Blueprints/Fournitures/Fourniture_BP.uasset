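; Fourniture_BP is a furniture actor that holds one object for taking or dropping, with text renders showing its name, content and ingredient count.
; DropContent stores objects when empty, or casts them to add ingredients to a held Deliverer_BP or exchange between two deliverers.
; A dropped Pocket_BP spawns a Biscuit_BP at a hardcoded location, flavored from the pocket and added to the deliverer.
; Debug functions print contents; Use is a stub.
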(event EventBeginPlay
  (CallFunction|Initialise))

(event Collision|EventActorBeginOverlap
  (params (OtherActor :type Actor%20Object%20Reference)))

(event EventTick
  (params (DeltaSeconds :type Float%20%28single-precision%29)))

(fn ConstructionScript)

(fn TakeontheTable
  (if (Utilities|IsValid (Variables|Default|GetObject))
    (LocalVariables|SetObjectToTake (Variables|Default|GetObject))
    (Variables|Default|SetObject 0)
    (CallFunction|SetDisplayObject)
    (return (LocalVariables|GetObjectToTake))))

(fn DropContent
  (params (Content :type Transportable%20BP%20Object%20Reference))
  (LocalVariables|SetObjectDropped Content)
  (if (Utilities|IsValid (Variables|Default|GetObject))
    (bind _asdeliverer_bp (Utilities|Casting|CastToDeliverer_BP (Variables|Default|GetObject))
      (:then
        (bind _asingredient_bp (Utilities|Casting|CastToIngredient_BP (LocalVariables|GetObjectDropped))
          (:then
            (bind _added (Default|AddIngredient _asdeliverer_bp _asingredient_bp))
            (CallFunction|SetDisplayObject)
            (return _added))
          (:CastFailed
            (bind _aspocket_bp (Utilities|Casting|CastToPocket_BP (LocalVariables|GetObjectDropped))
              (:then
                (bind _dropped (CallFunction|MakeBiscuit _aspocket_bp))
                (CallFunction|SetDisplayObject)
                (return _dropped))
              (:CastFailed
                (bind _asdeliverer_bp_2 (Utilities|Casting|CastToDeliverer_BP (LocalVariables|GetObjectDropped))
                  (:then
                    (bind _succeed (Default|Exchange _asdeliverer_bp _asdeliverer_bp_2 _asdeliverer_bp))
                    (CallFunction|SetDisplayObject)
                    (return _succeed))
                  (:CastFailed
                    (return false))))))))
      (:CastFailed
        (Development|PrintString "Already an object." true true "(R=1.000000,G=0.000000,B=0.000000,A=1.000000)")
        (return false)))
    (else
      (Variables|Default|SetObject (LocalVariables|GetObjectDropped))
      (CallFunction|SetDisplayObject)
      (return true))))

(fn Initialise
  (Rendering|Components|TextRender|SetText (Variables|Default|GetTextRender) (Variables|Default|GetName))
  (CallFunction|SetDisplayObject))

(fn TakeContent
  (bind _content (CallFunction|TakeontheTable))
  (return _content))

(fn SetDisplayObject
  (if (Utilities|IsValid (Variables|Default|GetObject))
    (LocalVariables|SetDisplayObject (Variables|/Game/EpiLib/Blueprints/Objects/Transportable_BP.Transportable_BP_C|GetName (Variables|Default|GetObject)))
    (bind _asdeliverer_bp (Utilities|Casting|CastToDeliverer_BP (Variables|Default|GetObject))
      (:then
        (LocalVariables|SetDisplayIngredientDeliverer (Utilities|Text|ToText(Integer) (Utilities|Array|Length (Variables|/Game/EpiLib/Blueprints/Objects/Deliverer_BP.Deliverer_BP_C|GetIngredient _asdeliverer_bp)))))
      (:CastFailed
        (LocalVariables|SetDisplayIngredientDeliverer "")))
    (else
      (LocalVariables|SetDisplayObject "")
      (LocalVariables|SetDisplayIngredientDeliverer "")))
  (Rendering|Components|TextRender|SetText (Variables|Default|GetObjectTextRender) (LocalVariables|GetDisplayObject))
  (Rendering|Components|TextRender|SetText (Variables|Default|GetDelivererTextRender) (LocalVariables|GetDisplayIngredientDeliverer)))

(fn Debug
  (bind _output_get (LocalVariables|SetNameString (Utilities|String|Append "Name:" (Utilities|String|ToString(Text) (Variables|Default|GetName)))))
  (Development|PrintString _output_get true true "(R=0.000000,G=0.660000,B=1.000000,A=1.000000)" 5.0)
  (CallFunction|DebugObject))

(fn DebugObject
  (if (Utilities|IsValid (Variables|Default|GetObject))
    (bind _asingredient_bp (Utilities|Casting|CastToIngredient_BP (Variables|Default|GetObject))
      (:then
        (Development|PrintString (Utilities|String|Append (LocalVariables|GetObjectDisplay) "[Ingredient] " (Utilities|String|ToString(Text) (Variables|/Game/EpiLib/Blueprints/Objects/Transportable_BP.Transportable_BP_C|GetName _asingredient_bp))) true true "(R=0.000000,G=0.660000,B=1.000000,A=1.000000)" 5.0))
      (:CastFailed
        (bind _asdeliverer_bp (Utilities|Casting|CastToDeliverer_BP (Variables|Default|GetObject)))
        (Development|PrintString (Utilities|String|Append (LocalVariables|GetObjectDisplay) (Utilities|String|ToString(Text) (Variables|/Game/EpiLib/Blueprints/Objects/Transportable_BP.Transportable_BP_C|GetName _asdeliverer_bp)) ":") true true "(R=0.000000,G=0.660000,B=1.000000,A=1.000000)" 5.0)
        (if (!= (Utilities|Array|Length (Variables|/Game/EpiLib/Blueprints/Objects/Deliverer_BP.Deliverer_BP_C|GetIngredient _asdeliverer_bp)) 0)
          (for _array_element (Variables|/Game/EpiLib/Blueprints/Objects/Deliverer_BP.Deliverer_BP_C|GetIngredient _asdeliverer_bp)
            (Development|PrintString (Utilities|String|ToString(Text) (Variables|/Game/EpiLib/Blueprints/Objects/Transportable_BP.Transportable_BP_C|GetName _array_element)) true true "(R=0.000000,G=0.660000,B=1.000000,A=1.000000)" 5.0))
          (else
            (Development|PrintString "NULL" true true "(R=0.000000,G=0.660000,B=1.000000,A=1.000000)" 5.0)))))
    (else
      (Development|PrintString (Utilities|String|Append (LocalVariables|GetObjectDisplay) "NULL") true true "(R=0.000000,G=0.660000,B=1.000000,A=1.000000)" 5.0))))

(fn Use
  (params (TransportedTool :type Tool%20BP%20Object%20Reference))
  (bind _output_get (LocalVariables|SetTool TransportedTool))
  (if (Utilities|IsValid _output_get)
    (Utilities|Casting|CastToBowl_BP (Variables|Default|GetObject))))

(fn MakeBiscuit
  (params (TransportedObject :type Pocket%20BP%20Object%20Reference))
  (LocalVariables|SetPocket TransportedObject)
  (bind _returnvalue (Game|SpawnActorfromClass "/Game/EpiLib/Blueprints/Objects/Ingredients/Biscuit_BP.Biscuit_BP_C" (Math|Transform|MakeTransform "-880.000000,-700.000000,-190.000000" "0, 0, 0" "1,1,1") "AlwaysSpawn" 0 0))
  (bind _output_get (LocalVariables|SetBiscuit _returnvalue))
  (Variables|/Game/EpiLib/Blueprints/Objects/Ingredients/Biscuit_BP.Biscuit_BP_C|SetFlavor _output_get (Variables|/Game/EpiLib/Blueprints/Objects/Deliverer_BP.Deliverer_BP_C|GetIngredient (LocalVariables|GetPocket)))
  (Variables|/Game/EpiLib/Blueprints/Objects/Transportable_BP.Transportable_BP_C|SetName (LocalVariables|GetBiscuit) "Biscuit")
  (bind _asdeliverer_bp (Utilities|Casting|CastToDeliverer_BP (Variables|Default|GetObject)))
  (bind _added (Default|AddIngredient _asdeliverer_bp (LocalVariables|GetBiscuit)))
  (return _added))