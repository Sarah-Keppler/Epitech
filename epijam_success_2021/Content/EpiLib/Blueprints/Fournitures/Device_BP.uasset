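; Device_BP is a furniture device that holds one Deliverer container and turns its ingredients into recipe results.
; DropContent stores a Deliverer, even if its class is disallowed, or adds an Ingredient to the held one; TakeContent removes the Deliverer.
; Use tries recipes until one matches by ingredient count and class, yielding a result ingredient or a copied Deliverer carrying the ingredients.
; A text render shows the ingredient count.
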(event EventBeginPlay
  (|CallParentFunction)
  (CallFunction|SetDisplayObject))

(event Collision|EventActorBeginOverlap
  (params (OtherActor :type Actor%20Object%20Reference))
  (|CallParentFunction OtherActor) ; This node is disabled and will not be called.\nDrag off pins to build functionality.
)

(event EventTick
  (params (DeltaSeconds :type Float%20%28single-precision%29))
  (|CallParentFunction DeltaSeconds) ; This node is disabled and will not be called.\nDrag off pins to build functionality.
)

(fn ConstructionScript
  (|CallParentFunction))

(fn TakeContent
  (if (Utilities|IsValid (Variables|Default|GetDeliverer))
    (LocalVariables|SetDelivererToTake (Variables|Default|GetDeliverer))
    (Variables|Default|SetDeliverer 0)
    (CallFunction|SetDisplayObject)
    (Development|PrintString (Utilities|String|ToString(Boolean) (Utilities|IsValid (Variables|Default|GetDeliverer))))
    (return (LocalVariables|GetDelivererToTake))))

(fn DropContent
  (params (Content :type Transportable%20BP%20Object%20Reference))
  (bind _output_get (LocalVariables|SetNewContent Content))
  (bind _asdeliverer_bp (Utilities|Casting|CastToDeliverer_BP _output_get)
    (:then
      (if (Utilities|IsValid (Variables|Default|GetDeliverer))
        (return false)
        (else
          (Development|PrintString "Hello")
          (bind _output_get_2 (LocalVariables|SetNewDeliverer _asdeliverer_bp))
          (bind _allowed (CallFunction|IsAllowedDeliverer _output_get_2))
          (Development|PrintString (Utilities|String|ToString(Boolean) _allowed))
          (Variables|Default|SetDeliverer (LocalVariables|GetNewDeliverer))
          (CallFunction|SetDisplayObject)
          (return _allowed))))
    (:CastFailed
      (bind _asingredient_bp (Utilities|Casting|CastToIngredient_BP (LocalVariables|GetNewContent))
        (:then
          (if (Utilities|IsValid (Variables|Default|GetDeliverer))
            (bind _added (Default|AddIngredient (Variables|Default|GetDeliverer) _asingredient_bp))
            (CallFunction|SetDisplayObject)
            (return _added)
            (else
              (return false))))
        (:CastFailed
          (return false))))))

(fn IsAllowedDeliverer
  (params (Deliverer :type Deliverer%20BP%20Object%20Reference))
  (return (!= (Utilities|Array|FindItem (Variables|Default|GetAllowedDeliverers) (Utilities|GetClass Deliverer)) -1)))

(fn SetDisplayObject
  (if (Utilities|IsValid (Variables|Default|GetDeliverer))
    (LocalVariables|SetDisplay (Utilities|Text|ToText(Integer) (Utilities|Array|Length (Variables|/Game/EpiLib/Blueprints/Objects/Deliverer_BP.Deliverer_BP_C|GetIngredient (Variables|Default|GetDeliverer)))))
    (else
      (LocalVariables|SetDisplay "")))
  (Rendering|Components|TextRender|SetText (Variables|Default|GetDelivererTextRender) (LocalVariables|GetDisplay)))

(fn Debug
  (bind _deliverer (Variables|Default|GetDeliverer))
  (bind _ingredient (Variables|/Game/EpiLib/Blueprints/Objects/Deliverer_BP.Deliverer_BP_C|GetIngredient _deliverer))
  (Development|PrintString (Utilities|String|Append "Name:" (Utilities|String|ToString(Text) (Variables|Default|GetName))) true true "(R=0.000000,G=0.660000,B=1.000000,A=1.000000)" 5.0)
  (if (Utilities|IsValid (Variables|Default|GetDeliverer))
    (Development|PrintString (Utilities|String|Append (LocalVariables|GetDelivererDIsplay) (Utilities|String|ToString(Text) (Variables|/Game/EpiLib/Blueprints/Objects/Transportable_BP.Transportable_BP_C|GetName _deliverer)) ":") true true "(R=0.000000,G=0.660000,B=1.000000,A=1.000000)" 5.0)
    (if (!= (Utilities|Array|Length _ingredient) 0)
      (for _array_element _ingredient
        (Development|PrintString (Utilities|String|ToString(Text) (Variables|/Game/EpiLib/Blueprints/Objects/Transportable_BP.Transportable_BP_C|GetName _array_element)) true true "(R=0.000000,G=0.660000,B=1.000000,A=1.000000)" 5.0))
      (else
        (Development|PrintString "NULL" true true "(R=0.000000,G=0.660000,B=1.000000,A=1.000000)" 5.0)))
    (else
      (Development|PrintString (Utilities|String|Append (LocalVariables|GetDelivererDIsplay) "NULL") true true "(R=0.000000,G=0.660000,B=1.000000,A=1.000000)" 5.0))))

(fn Use
  (params (TransportedTool :type Tool%20BP%20Object%20Reference))
  (for _array_element (Variables|Default|GetRecipes)
    (if (not (LocalVariables|GetBreak))
      (bind _succeed (CallFunction|MakeRecipe _array_element))
      (LocalVariables|SetBreak _succeed)))
  (CallFunction|SetDisplayObject))

(fn MakeRecipe
  (params (Recipe :type Recipe%20S%20Structure))
  (bind _ingredientsavailableclasses (LocalVariables|GetIngredientsAvailableClasses))
  (LocalVariables|SetGivenRecipe Recipe)
  (if (Utilities|IsValid (Variables|Default|GetDeliverer))
    (bind _output_get (LocalVariables|SetIngredientsAvailable (Variables|/Game/EpiLib/Blueprints/Objects/Deliverer_BP.Deliverer_BP_C|GetIngredient (Variables|Default|GetDeliverer))))
    (if (and (!= 0 (Utilities|Array|Length _output_get)) (== (Utilities|Array|Length _output_get) (Utilities|Array|Length (.ressources (LocalVariables|GetGivenRecipe)))))
      (for _array_element (LocalVariables|GetIngredientsAvailable)
        (Utilities|Array|AddUnique (LocalVariables|GetIngredientsAvailableClasses) (Utilities|GetClass _array_element)))
      (for _array_element_2 (.ressources (LocalVariables|GetGivenRecipe))
        (Utilities|Array|RemoveItem _ingredientsavailableclasses (Utilities|Array|Get(acopy) _ingredientsavailableclasses (Utilities|Array|FindItem _ingredientsavailableclasses _array_element_2))))
      (if (== (Utilities|Array|Length _ingredientsavailableclasses) 0)
        (bind _asingredient_bp (Utilities|Casting|CastToIngredient_BP (.result (LocalVariables|GetGivenRecipe)))
          (:then
            (Default|Clear (Variables|Default|GetDeliverer))
            (bind _added (Default|AddIngredient (Variables|Default|GetDeliverer) _asingredient_bp))
            (return _added))
          (:CastFailed
            (bind _asdeliverer_bp (Utilities|Casting|CastToDeliverer_BP (.result (LocalVariables|GetGivenRecipe))))
            (bind _copy (Default|GetACopy _asdeliverer_bp _asdeliverer_bp))
            (bind _asdeliverer_bp_2 (Utilities|Casting|CastToDeliverer_BP _copy))
            (LocalVariables|SetCopy _asdeliverer_bp_2)
            (for _array_element_3 (LocalVariables|GetIngredientsAvailable)
              (bind _added_2 (Default|AddIngredient (LocalVariables|GetCopy) _array_element_3))
              (if (not _added_2)
                (return false)))
            (Variables|Default|SetDeliverer (LocalVariables|GetCopy))
            (return true)))
        (else
          (return false)))
      (else
        (return false)))
    (else
      (return false))))