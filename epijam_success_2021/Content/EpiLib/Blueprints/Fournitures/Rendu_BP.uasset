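; Rendu_BP is a supply actor that serves as a drop-off point where plates are turned in for money.
; On BeginPlay it runs the parent logic, then writes Value to its text render label.
; DropContent accepts only an Assiette_BP, calls its Valid function and returns that result.
; It adds a fixed 150 to the first player character's Money without branching on the validation result.
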(event EventBeginPlay
  (|CallParentFunction)
  (Rendering|Components|TextRender|SetText (Variables|Default|GetObjectTextRender) (Variables|Default|GetValue)))

(event Collision|EventActorBeginOverlap
  (params (OtherActor :type Actor%20Object%20Reference))
  (|CallParentFunction OtherActor) ; This node is disabled and will not be called.\nDrag off pins to build functionality.
)

(event EventTick
  (params (DeltaSeconds :type Float%20%28single-precision%29))
  (|CallParentFunction DeltaSeconds) ; This node is disabled and will not be called.\nDrag off pins to build functionality.
)

(fn ConstructionScript
  (|CallParentFunction))

(fn DropContent
  (params (Content :type Transportable%20BP%20Object%20Reference))
  (bind _asassiette_bp (Utilities|Casting|CastToAssiette_BP Content))
  (bind _isvalid (Default|Valid _asassiette_bp))
  (bind _ascharacter_bp (Utilities|Casting|CastToCharacter_BP (Game|GetPlayerCharacter 0)))
  (Variables|/Game/EpiLib/Blueprints/Characters/Character_BP.Character_BP_C|SetMoney _ascharacter_bp (+ (Variables|/Game/EpiLib/Blueprints/Characters/Character_BP.Character_BP_C|GetMoney _ascharacter_bp) 150))
  (return _isvalid))