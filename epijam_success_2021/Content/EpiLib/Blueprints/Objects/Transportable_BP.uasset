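; Transportable object actor in EpiLib that displays its Name on a text render component, set through Initialise on BeginPlay.
; GetACopy duplicates a given transportable by spawning its runtime class at a hard-coded location, ignoring collisions, then copies only Name and returns the new actor.
; Name is assigned after the spawn call, and the function does not refresh the text itself.
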(event EventBeginPlay
  (CallFunction|Initialise))

(event Collision|EventActorBeginOverlap
  (params (OtherActor :type Actor%20Object%20Reference)))

(event EventTick
  (params (DeltaSeconds :type Float%20%28single-precision%29)))

(fn ConstructionScript)

(fn Initialise
  (Rendering|Components|TextRender|SetText (Variables|Default|GetTextRender) (Variables|Default|GetName)))

(fn GetACopy
  (params (Original :type Transportable%20BP%20Object%20Reference))
  (bind _output_get (LocalVariables|SetPreCopy Original))
  (bind _returnvalue (Game|SpawnActorfromClass (Utilities|GetClass _output_get) (Math|Transform|MakeTransform "-880.000000,-700.000000,-190.000000" "0, 0, 0" "1,1,1") "AlwaysSpawn" 0 0))
  (Variables|Transportable_BP_C|SetName _returnvalue (Variables|Transportable_BP_C|GetName (LocalVariables|GetPreCopy)))
  (return _returnvalue))