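; Assiette_BP is a plate actor in the Deliverers folder that collects ingredients for a recipe (Recette).
; AddIngredient accepts an ingredient only if its class is in Recette and not already in ContentClass, then records both class and instance and returns whether it succeeded.
; Valid reports completion by comparing the Recette and ContentClass lengths, so each ingredient class counts once.
; The event graph holds only disabled default events.
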(event EventBeginPlay
  (|CallParentFunction) ; This node is disabled and will not be called.\nDrag off pins to build functionality.
)

(event Collision|EventActorBeginOverlap
  (params (OtherActor :type Actor%20Object%20Reference))
  (|CallParentFunction OtherActor) ; This node is disabled and will not be called.\nDrag off pins to build functionality.
)

(event EventTick
  (params (DeltaSeconds :type Float%20%28single-precision%29))
  (|CallParentFunction DeltaSeconds) ; This node is disabled and will not be called.\nDrag off pins to build functionality.
)

(fn ConstructionScript
  (|CallParentFunction))

(fn AddIngredient
  (params (Ingredient :type Ingredient%20BP%20Object%20Reference))
  (bind _output_get (LocalVariables|SetNew%20Ingredient Ingredient))
  (if (!= (Utilities|Array|FindItem (Variables|Default|GetRecette) (Utilities|GetClass _output_get)) -1)
    (if (== (Utilities|Array|FindItem (Variables|Default|GetContentClass) (Utilities|GetClass (LocalVariables|GetNew%20Ingredient))) -1)
      (Utilities|Array|Add (Variables|Default|GetContentClass) (Utilities|GetClass (LocalVariables|GetNew%20Ingredient)))
      (Utilities|Array|Add (Variables|Default|GetIngredient) (LocalVariables|GetNew%20Ingredient))
      (return true)
      (else
        (return false)))
    (else
      (return false))))

(fn Valid
  (return (== (Utilities|Array|Length (Variables|Default|GetRecette)) (Utilities|Array|Length (Variables|Default|GetContentClass)))))