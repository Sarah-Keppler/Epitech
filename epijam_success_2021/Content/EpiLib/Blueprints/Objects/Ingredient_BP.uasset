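; Ingredient_BP is an ingredient object that reports when it is taken or dropped.
; IsTaken and IsDropped each print an on-screen debug message built from the Name value and the new state.
; The event graph holds only disabled default events and the construction script just calls its parent, so no other logic runs here.
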(event EventBeginPlay
  (|CallParentFunction) ; This node is disabled and will not be called.\nDrag off pins to build functionality.
)

(event Collision|EventActorBeginOverlap
  (params (OtherActor :type Actor%20Object%20Reference))
  (|CallParentFunction OtherActor) ; This node is disabled and will not be called.\nDrag off pins to build functionality.
)

(event EventTick
  (params (DeltaSeconds :type Float%20%28single-precision%29))
  (|CallParentFunction DeltaSeconds) ; This node is disabled and will not be called.\nDrag off pins to build functionality.
)

(fn ConstructionScript
  (|CallParentFunction))

(fn IsTaken
  (Development|PrintString (Utilities|String|Append (Utilities|String|ToString(Text) (Variables|Default|GetName)) " is taken.") true true "(R=1.000000,G=0.631373,B=0.145098,A=1.000000)"))

(fn IsDropped
  (Development|PrintString (Utilities|String|Append (Utilities|String|ToString(Text) (Variables|Default|GetName)) " is dropped.") true true "(R=1.000000,G=0.631373,B=0.145098,A=1.000000)"))